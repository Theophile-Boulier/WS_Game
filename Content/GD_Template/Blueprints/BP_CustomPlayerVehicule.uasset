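; BP_CustomPlayerVehicule is a wheeled vehicle Blueprint with checkpoint respawning and a selectable control type.
; BeginPlay stores the starting transform as the respawn point, which SetRespawnPosition can replace, and RaceStart flags the race as started.
; Respawn teleports to that point, optionally zeroing velocity with a brief handbrake; the last-checkpoint input keeps velocity.
; The construction script sets back spring arm length from ControlType, while RPM-based engine pitch logic is left unconnected.
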(event `self.ReceiveBeginPlay`
  (`parent.ReceiveBeginPlay`)
  (`self.SetRespawnPosition` (`self.GetTransform`))
  (if (`self.bIsPlayer`)
    _))

(event `Respawn`
  (params (KeepVelocity :type Boolean))
  (bind (_lastrespawnposition_location _lastrespawnposition_rotation) (`KismetMathLibrary.BreakTransform` (`self.LastRespawnPosition`)))
  (`self.K2_SetActorTransform` (`KismetMathLibrary.MakeTransform` _lastrespawnposition_location _lastrespawnposition_rotation) false true)
  (if (not KeepVelocity)
    (`ChaosVehicleMovementComponent.SetHandbrakeInput` (`self.VehicleMovementComponent`) true)
    (`PrimitiveComponent.SetAllPhysicsLinearVelocity` (`self.Mesh`) (0.0 0.0 0.0) false)
    (`KismetSystemLibrary.Delay` 0.2)
    (`ChaosVehicleMovementComponent.SetHandbrakeInput` (`self.VehicleMovementComponent`) false)))

(event `RaceStart`
  (set `self.bIsRaceStarted` true))

(event `self.ReceiveTick`
  (params (DeltaSeconds :type "Float (single-precision)"))
  ;[1 1 1] SpeedSound
)

(event `EnhancedInput|/Game/GD_Template/VehicleTemplate/Input/Actions/IA_LastCheckpoint`
  (params (ActionValue :type Boolean) (ElapsedSeconds :type "Float (double-precision)") (TriggeredSeconds :type "Float (double-precision)") (InputAction :type "InputAction Object Reference" :default "/Game/GD_Template/VehicleTemplate/Input/Actions/IA_LastCheckpoint.IA_LastCheckpoint"))
  (:`Triggered`
    (`self.Respawn` true)))

(fn `ControlParameters`
  (params (`Target Arm Length` :type "Float (single-precision)"))
  (set `SpringArmComponent.TargetArmLength` `Target Arm Length` (`self.BackSpringArm`)))

(fn `SetRespawnPosition`
  (params (RespawnPos :type "Transform Structure"))
  (set `self.LastRespawnPosition` RespawnPos))

(fn `UserConstructionScript`
  (`parent.UserConstructionScript`)
  (switch `/Game/GD_Template/Datas/E_ControlPresets` (`self.ControlType`)
    (:`NewEnumerator0`
      (`self.ControlParameters` 650.0))
    (:`NewEnumerator1`
      (`self.ControlParameters` 0.0))
    (:`NewEnumerator2`
      (`self.ControlParameters` 0.0))))