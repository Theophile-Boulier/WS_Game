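; Finish line actor for a lap-based race, validating player laps and recording the arrival order of cars.
; It registers itself with RaceManager, collects checkpoints that add themselves, and sets their total one tick after BeginPlay.
; When the player overlaps its box, RaceManager either finishes the lap or flags a missed checkpoint.
; AI drivers count laps without checkpoint checks, and a player arrival sends the leaderboard to RaceManager to end the game.
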(event `PrepareNextTurn`
  ;[1 1 1] Reset les checkpoint pour le prochain tour
  (for _array_element (`self.AllCheckpoint`)
    (set `/Game/GD_Template/Race/BP_CheckPoint.Passed` false _array_element)
    (set `/Game/GD_Template/Race/BP_RaceManager.CheckpointCount` 0 (`self.RaceManager`))))

(event `self.ReceiveBeginPlay`
  ;[1 1 1] Init
  (set `/Game/GD_Template/Race/BP_RaceManager.FinishLine` self (`self.RaceManager`))
  (`KismetSystemLibrary.DelayUntilNextTick`)
  (set `/Game/GD_Template/Race/BP_RaceManager.CheckpointMaxCount` (`KismetArrayLibrary.Array_Length` (`self.AllCheckpoint`)) (`self.RaceManager`)))

(event `AddCheckpointToList`
  (params (CheckpointToAdd :type "/Game/GD_Template/Race/BP_CheckPoint Object Reference"))
  ;[1 1 1] Init
  (`KismetArrayLibrary.Array_Add` (`self.AllCheckpoint`) CheckpointToAdd))

(event `PassCheckpoint`
  (bind _racemanager (`self.RaceManager`))
  ;[1 1 1] Passer un checkpoint
  (set `/Game/GD_Template/Race/BP_RaceManager.CheckpointCount` (+ (`/Game/GD_Template/Race/BP_RaceManager.CheckpointCount` _racemanager) 1) _racemanager))

(event `self.BoxCollision.OnComponentBeginOverlap`
  (params (OverlappedComponent :type "PrimitiveComponent Object Reference") (OtherActor :type "Actor Object Reference") (OtherComp :type "PrimitiveComponent Object Reference") (OtherBodyIndex :type Integer) (bFromSweep :type Boolean) (SweepResult :type "HitResult Structure (by ref)"))
  (bind _racemanager (`self.RaceManager`))
  (bind _racemanager_2 (`self.RaceManager`))
  ;[1 1 1] Passer la ligne d'arrivée
  (if (== OtherActor (`GameplayStatics.GetPlayerPawn` 0))
    (if (== (`/Game/GD_Template/Race/BP_RaceManager.CheckpointCount` _racemanager) (`/Game/GD_Template/Race/BP_RaceManager.CheckpointMaxCount` _racemanager))
      (`/Game/GD_Template/Race/BP_RaceManager.FinishLap` _racemanager_2)
      (else
        (`/Game/GD_Template/Race/BP_RaceManager.MissingACheckpoint` _racemanager_2)))
    (else
      (bind _asbp_driver_ai (cast `/Game/GD_Template/Blueprints/BP_DriverAI` OtherActor))
      (bind _output_get (set `/Game/GD_Template/Blueprints/BP_DriverAI.LapNumber` (+ (`/Game/GD_Template/Blueprints/BP_DriverAI.LapNumber` _asbp_driver_ai) 1) _asbp_driver_ai))
      (if (== _output_get (`/Game/GD_Template/Race/BP_RaceManager.NombreDeToursMax` (`self.RaceManager`)))
        (`self.AddToLeaderboard` _asbp_driver_ai)))))

(event `AddToLeaderboard`
  (params (`Arrived Car` :type "/Game/GD_Template/Blueprints/BP_CustomPlayerVehicule Object Reference") (IsPlayer :type Boolean))
  (`KismetArrayLibrary.Array_Add` (`self.ArrivedCars`) `Arrived Car`)
  (if IsPlayer
    (`/Game/GD_Template/Race/BP_RaceManager.OnEndGame` (`self.RaceManager`) (`self.ArrivedCars`))))

(fn `UserConstructionScript`)